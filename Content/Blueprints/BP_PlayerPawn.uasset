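; BP_PlayerPawn is the player pawn Blueprint that owns the player's UI: HUD, crosshair, bloody-screen health overlay and pause menu.
; BeginPlay creates the widgets, adding the HUD and initially hidden crosshair to the viewport, but not the bloody screen.
; Events toggle the crosshair and forward health to HUD and overlay, stamina to HUD alone.
; PauseGame input lazily creates the menu and toggles pause, cursor and input mode.
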(event EventTick
  (params (DeltaSeconds :type Float%20%28single-precision%29))
  (Utilities|FlowControl|Sequence))

(event EventBeginPlay
  (bind _self self)
  (Utilities|FlowControl|Sequence
    (:then_0
      (Variables|Default|SetCharacterReference self))
    (:then_1
      (bind _returnvalue (Game|ConstructObjectfromClass "/Game/Blueprints/UI/WBP_BloodyScreen.WBP_BloodyScreen_C"))
      (Variables|Default|SetHealthScreen _returnvalue))
    (:then_2
      (bind _returnvalue_2 (Game|ConstructObjectfromClass _self "/Game/Blueprints/UI/WBP_Crosshair.WBP_Crosshair_C"))
      (bind _output_get (Variables|Default|SetCrosshair _returnvalue_2))
      (UserInterface|Viewport|AddtoViewport _output_get 0)
      (Widget|SetVisibility _output_get "Hidden"))
    (:then_3
      (bind _returnvalue_3 (Game|ConstructObjectfromClass _self "/Game/Blueprints/UI/WBP_HUD.WBP_HUD_C"))
      (bind _output_get_2 (Variables|Default|SetHUD _returnvalue_3))
      (UserInterface|Viewport|AddtoViewport _output_get_2 0))))

(event EventSetCrosshairActive
  (params (Active :type Boolean))
  (bind _crosshair (Variables|Default|GetCrosshair))
  (if Active
    (Widget|SetVisibility _crosshair "Visible")
    (else
      (Widget|SetVisibility _crosshair "Hidden"))))

(event EventUpdateHealth
  (params (UpdatedHealth :type Float%20%28single-precision%29))
  (Default|UpdateHealth (Variables|Default|GetHUD) UpdatedHealth)
  (Default|UpdateHealth (Variables|Default|GetHealthScreen) UpdatedHealth))

(event EventUpdateStamina
  (params (UpdatedStamina :type Float%20%28single-precision%29))
  ;[1 1 1] Update Stamina
  (Default|UpdateStamina (Variables|Default|GetHUD) UpdatedStamina))

(event Input|ActionEvents|InputActionPauseGame
  (params (Key :type Key%20Structure :default "None"))
  (bind _returnvalue (Game|GetPlayerController 0))
  ;[1 1 1] Pause/Unpause Menu
  (:Pressed
    (Utilities|IsValid (Variables|Default|GetPauseMenu)
      (:Is%20Valid
        _)
      (:Is%20Not%20Valid
        (bind _returnvalue_2 (UserInterface|CreateWidget "/Game/Blueprints/UI/WBP_PauseMenu.WBP_PauseMenu_C"))
        (Variables|Default|SetPauseMenu _returnvalue_2)))
    (if (Game|IsGamePaused)
      (Widget|RemovefromParent (Variables|Default|GetPauseMenu))
      (Game|SetGamePaused false)
      (Variables|/Script/Engine.PlayerController|SetbShowMouseCursor _returnvalue false)
      (Input|SetInputModeGameOnly _returnvalue false)
      (else
        (UserInterface|Viewport|AddtoViewport (Variables|Default|GetPauseMenu) 0)
        (Game|SetGamePaused true)
        (Variables|/Script/Engine.PlayerController|SetbShowMouseCursor _returnvalue true)
        (Input|SetInputModeGameandUI _returnvalue (Variables|Default|GetPauseMenu) "LockAlways" false false)))))

(fn ConstructionScript)