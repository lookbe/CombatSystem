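; Enemy AI actor that runs the BT_EnemyAI behavior tree and manages its own health bar and warning indicator.
; It stores the player pawn in the Blackboard on BeginPlay, then pushes its CurrentState and the player's location every Tick.
; The health bar shows while the enemy is lock-on targeted or briefly after a hit, with a timer restoring lock-based visibility.
; UpdateHealth forwards new values to the WBP_EnemyHealthbar widget.
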(event EventUpdateHealth
  (params (UpdatedHealth :type Float%20%28single-precision%29))
  (bind _aswbp_enemy_healthbar (Utilities|Casting|CastToWBP_EnemyHealthbar (UserInterface|GetUserWidgetObject (Variables|Default|GetHealthBar))))
  (Default|UpdateHealth _aswbp_enemy_healthbar UpdatedHealth))

(event EventOnHit
  (Rendering|SetVisibility (Variables|Default|GetHealthBar) true false)
  (bind _returnvalue (Utilities|Time|SetTimerbyFunctionName 0 "DisableHealthBar" (Variables|Default|GetTimeToDisableHealthBar)))
  (Variables|Default|SetHealthBarTimerHandle _returnvalue))

(event EventOnSetasTarget
  (params (IsTarget :type Boolean))
  (bind _output_get (Variables|Default|SetIsLockedTarget IsTarget))
  (Rendering|SetVisibility (Variables|Default|GetHealthBar) _output_get false))

(event EventBeginPlay
  (AI|RunBehaviorTree (AI|GetAIController self) "/Game/Blueprints/AI/BT_EnemyAI.BT_EnemyAI")
  (Utilities|FlowControl|Sequence
    (:then_0
      (bind _output_get (Variables|Default|SetBlackboard (AI|GetBlackboard self)))
      (bind _output_get_2 (Variables|Default|SetPlayer (Game|Player|GetPlayerPawn 0)))
      (AI|Components|Blackboard|SetValueasObject _output_get (Utilities|Name|MakeLiteralName "Player") _output_get_2))))

(event EventTick
  (params (DeltaSeconds :type Float%20%28single-precision%29))
  (Utilities|FlowControl|Sequence
    (:then_0
      (AI|Components|Blackboard|SetValueasEnum (Variables|Default|GetBlackboard) (Utilities|Name|MakeLiteralName "CurrentState") (Variables|Default|GetCurrentState self)))
    (:then_1
      (AI|Components|Blackboard|SetValueasVector (Variables|Default|GetBlackboard) (Utilities|Name|MakeLiteralName "TargetDestination") (Transformation|GetActorLocation (Variables|Default|GetPlayer))))))

(fn ConstructionScript)

(fn SetWarningIndicatorVisible
  (params (bNewVisibility :type Boolean))
  (Rendering|SetVisibility (Variables|Default|GetWarningIndicator) bNewVisibility false))

(fn DisableHealthBar
  (Rendering|SetVisibility (Variables|Default|GetHealthBar) (Variables|Default|GetIsLockedTarget) false)
  (Utilities|Time|ClearandInvalidateTimerbyHandle (Variables|Default|GetHealthBarTimerHandle)))