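; BP_DummyAI is a dummy AI enemy that manages its health bar and lock-on target indicator.
; Being set as the locked target shows or hides both the indicator and the health bar.
; A hit reveals the bar and starts a timer that later restores its visibility to the lock state.
; Health updates are forwarded to the WBP_EnemyHealthbar widget inside the bar's widget component.
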(event EventUpdateHealth
  (params (UpdatedHealth :type Float%20%28single-precision%29))
  (bind _aswbp_enemy_healthbar (Utilities|Casting|CastToWBP_EnemyHealthbar (UserInterface|GetUserWidgetObject (Variables|Default|GetHealthBar))))
  (Default|UpdateHealth _aswbp_enemy_healthbar UpdatedHealth))

(event EventOnHit
  (Rendering|SetVisibility (Variables|Default|GetHealthBar) true false)
  (bind _returnvalue (Utilities|Time|SetTimerbyFunctionName 0 "DisableHealthBar" (Variables|Default|GetTimeToDisableHealthBar)))
  (Variables|Default|SetHealthBarTimerHandle _returnvalue))

(event EventOnSetasTarget
  (params (IsTarget :type Boolean))
  (bind _output_get (Variables|Default|SetIsLockedTarget IsTarget))
  (Rendering|SetVisibility (Variables|Default|GetLockedTargetIndicator) _output_get false)
  (Rendering|SetVisibility (Variables|Default|GetHealthBar) IsTarget false))

(fn ConstructionScript)

(fn DisableHealthBar
  (Rendering|SetVisibility (Variables|Default|GetHealthBar) (Variables|Default|GetIsLockedTarget) false)
  (Utilities|Time|ClearandInvalidateTimerbyHandle (Variables|Default|GetHealthBarTimerHandle)))