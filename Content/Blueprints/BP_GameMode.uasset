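; Wave-based game mode Blueprint that spawns AI enemies and drives the wave HUD and death screen.
; SpawnNewEnemy runs an EQS query for a random top-25% location, then spawns and registers BP_Enemy_AI there on success.
; Wave and enemy events update the WBP_WaveInfo counter, passing the alive count into its KilledEnemies input.
; Game over creates or re-shows WBP_DeathScreen, while WaveStateChanged does nothing.
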(event Custom|OnQueryFinishedEvent_Event_0
  (params (QueryInstance :type Env%20Query%20Instance%20Blueprint%20Wrapper%20Object%20Reference) (QueryStatus :type EEnvQueryStatus%20Enum :default "Processing"))
  (switch Utilities|FlowControl|Switch|SwitchonEEnvQueryStatus QueryStatus
    (:Success
      (bind _resultlocations (AI|EQS|GetQueryResultsasLocations QueryInstance))
      (for _array_element _resultlocations
        (bind _returnvalue (Game|SpawnActorfromClass "/Game/Blueprints/AI/BP_Enemy_AI.BP_Enemy_AI_C" (Math|Transform|MakeTransform _array_element) "AdjustIfPossibleButAlwaysSpawn" "MultiplyWithRoot" 0 0))
        (Class|CSGameMode|AddEnemy _returnvalue)
        (bind _returnvalue_2 (Class|CSGameMode|GetAliveEnemies))
        (bind _returnvalue_3 (Class|CSGameMode|GetWaveEnemies))
        (Default|UpdateEnemiesAmount (Variables|Default|GetWaveCounter) _returnvalue_2 _returnvalue_3)))))

(event EventSpawnNewEnemy
  (bind _returnvalue (AI|EQS|RunEQSQuery "/Game/Blueprints/AI/EnvironmentQueries/EQS_FindSpawnLocation.EQS_FindSpawnLocation" self "RandomBest25Pct"))
  (EventDispatchers|AssignOnQueryFinishedEvent _returnvalue (delegate Custom|OnQueryFinishedEvent_Event_0)))

(event EventOnGameOver
  (Utilities|IsValid (Variables|Default|GetDeathScreen)
    (:Is%20Valid
      (Widget|SetVisibility (Variables|Default|GetDeathScreen) "Visible"))
    (:Is%20Not%20Valid
      (bind _returnvalue (UserInterface|CreateWidget "/Game/Blueprints/UI/WBP_DeathScreen.WBP_DeathScreen_C"))
      (bind _output_get (Variables|Default|SetDeathScreen _returnvalue))
      (UserInterface|Viewport|AddtoViewport _output_get 0))))

(event EventWaveStateChanged
  (params (NewState :type EWaveState%20Enum :default "WaitingToStart") (OldState :type EWaveState%20Enum :default "WaitingToStart")))

(event EventBeginPlay
  (bind _returnvalue (UserInterface|CreateWidget "/Game/Blueprints/UI/WBP_WaveInfo.WBP_WaveInfo_C"))
  (bind _output_get (Variables|Default|SetWaveCounter _returnvalue))
  (UserInterface|Viewport|AddtoViewport _output_get 0)
  (Default|SetWave _output_get 1))

(event EventOnWaveStarted
  (Default|SetWave (Variables|Default|GetWaveCounter) (Variables|Default|GetWaveCount)))

(event EventUpdateEnemiesCounter
  (bind _returnvalue (Class|CSGameMode|GetAliveEnemies))
  (bind _returnvalue_2 (Class|CSGameMode|GetWaveEnemies))
  (Default|UpdateEnemiesAmount (Variables|Default|GetWaveCounter) _returnvalue _returnvalue_2))

(fn ConstructionScript)